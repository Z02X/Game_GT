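; Child NPC Blueprint for Rada Bancroft that adds a time-of-day gate to the inherited waypoint ordering.
; Its WaypointOrderController override reads the hour from the SimpleSky reference and defers to the parent logic from 4.75 onward.
; At earlier hours it returns the incoming waypoint ID unchanged.
; The event graph and construction script add no behavior of their own.
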(event `self.ReceiveBeginPlay`
  (`parent.ReceiveBeginPlay`))

(event `self.ReceiveActorBeginOverlap`
  (params (OtherActor :type "Actor Object Reference")))

(event `self.ReceiveTick`
  (params (DeltaSeconds :type "Float (single-precision)"))
  (`parent.ReceiveTick` 0.0))

(fn `UserConstructionScript`
  (`parent.UserConstructionScript`))

(fn `WaypointOrder_Controller`
  (params (IdIn :type Integer))
  (returns (IdOut :type Integer))
  (bind _assimple_sky (cast `/Game/Blueprints/SimpleSky` (`self.SimpleSkyRef`)))
  (if (>= (`/Game/Blueprints/SimpleSky.Hour` _assimple_sky) 4.75)
    (bind _idout (`parent.WaypointOrder_Controller` IdIn))
    (return _idout)
    (else
      (return IdIn))))