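; Test NPC actor that walks along a spline on a schedule driven by the hour from a SimpleSky actor.
; Each tick it advances by Speed from early morning, holds partway until evening, and resets at the path's end; Interrupted pauses it before then.
; A line trace from the spline point toward a fixed low Z sets its height just above the ground.
; It also prints the current hour every tick.
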(event `self.ReceiveBeginPlay`
  (bind _output_get (set `self.StartingLocation` (`self.K2_GetActorLocation`))))

(event `self.ReceiveTick`
  (params (DeltaSeconds :type "Float (single-precision)"))
  (bind _current_location (`self.Current Location`))
  (bind _assimple_sky (cast `/Game/Blueprints/SimpleSky` (`self.SkyControlerRef`)))
  (bind _hour (`/Game/Blueprints/SimpleSky.Hour` _assimple_sky))
  (bind _output_get (set `self.LocalHour` _hour))
  (`KismetSystemLibrary.PrintString` (`KismetStringLibrary.Conv_DoubleToString` _hour))
  (if (>= (`self.DistanceAlongSpline`) 1172.0)
    (set `self.DistanceAlongSpline` 0.0)
    (`self.K2_SetActorLocation` (stale `self.ReceiveBeginPlay` _output_get))
    (set `self.DistanceAlongSpline` (+ (`self.Speed`) (`self.DistanceAlongSpline`)) :!label _label)
    (set `self.Current Location` (`SplineComponent.GetLocationAtDistanceAlongSpline` (`/Game/Blueprints/SplineComponet.Spline` (`self.Spline_Blueprint`)) (`self.DistanceAlongSpline`) "World"))
    (bind _outhit (`KismetSystemLibrary.LineTraceSingleForObjects` _current_location (`KismetMathLibrary.MakeVector` (.x _current_location) (.y _current_location) 20.0) (`|MakeArray` "ObjectTypeQuery1" :!type "EObjectTypeQuery Enum")))
    (set `self.Trace Hit Location` (`.ImpactPoint` (`GameplayStatics.BreakHitResult` _outhit)))
    (`self.K2_SetActorLocation` (`KismetMathLibrary.MakeVector` (.x (`self.Current Location`)) (.y (`self.Current Location`)) (+ (.z (`self.Trace Hit Location`)) 20.0)))
    (elif (`self.Interrupted`)
      _
      (elif (>= _output_get 4.75)
        (if (>= (`self.DistanceAlongSpline`) 600.0)
          (if (>= (`self.LocalHour`) 18.0)
            (goto _label))
          (else
            (goto _label)))))))

(fn `GetLocationAtDistanceAlongSpline`
  (params (Target :type "SplineComponent Object Reference") (Distance :type "Float (double-precision)"))
  (returns (`Return Value` :type "Vector Structure"))
  (return (`SceneComponent.K2_GetComponentLocation` Target)))

(fn `UserConstructionScript`)