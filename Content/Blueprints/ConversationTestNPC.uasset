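; Test NPC for dialogue and punch interactions with the LizardMan Paper2D player.
; Construction tilts it and derives health from stats; overlapping PunchBox actors are destroyed, each costing one health, with only the first printed.
; Its sphere toggles an image on the player's HUD when meeting their DialogueBox.
; Helpers for grab-following and health bar updates are never called here; the damage calculator is disabled and regen is unwired.
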(event `self.ReceiveActorBeginOverlap`
  (params (OtherActor :type "Actor Object Reference"))
  (bind _currenthealth (`self.CurrentHealth`))
  (bind _aspunch_box (cast `/Game/Blueprints/PunchBox` OtherActor))
  (`self.K2_DestroyActor` _aspunch_box)
  (set `self.CurrentHealth` (- _currenthealth 1))
  (if (not (`self.Interrupted`))
    (set `self.Interrupted` true)
    (`KismetSystemLibrary.PrintString` (`KismetStringLibrary.Conv_IntToString` _currenthealth) true true (struct :`R` 1.0 :`G` 0.086053 :`B` 0.357803 :`A` 1.0))))

(event `self.Sphere.OnComponentBeginOverlap`
  (params (OtherActor :type "Actor Object Reference") (OtherComp :type "PrimitiveComponent Object Reference") (OtherBodyIndex :type Integer) (bFromSweep :type Boolean) (SweepResult :type "HitResult Structure (by ref)"))
  (bind _returnvalue (`GameplayStatics.GetPlayerCharacter` 0))
  (if (== _returnvalue OtherActor)
    (bind _aslizard_man_paper_character (cast `/Game/Blueprints/LizardMan_PaperCharacter` _returnvalue))
    (if (== OtherComp (`/Game/Blueprints/LizardMan_PaperCharacter.Dialogue Box` _aslizard_man_paper_character))
      (`Widget.SetVisibility` (`/Game/Blueprints/HPBar.Image_36` (`/Game/Blueprints/LizardMan_PaperCharacter.HPBar Widget` _aslizard_man_paper_character)) "Visible"))))

(event `self.Sphere.OnComponentEndOverlap`
  (params (OtherActor :type "Actor Object Reference") (OtherComp :type "PrimitiveComponent Object Reference") (OtherBodyIndex :type Integer))
  (if (== OtherActor (`GameplayStatics.GetPlayerCharacter` 0))
    (if (== OtherComp (`/Game/Blueprints/LizardMan_PaperCharacter.Dialogue Box` (stale `self.Sphere.OnComponentBeginOverlap` _aslizard_man_paper_character)))
      (`Widget.SetVisibility` (`/Game/Blueprints/HPBar.Image_36` (`/Game/Blueprints/LizardMan_PaperCharacter.HPBar Widget` (stale `self.Sphere.OnComponentBeginOverlap` _aslizard_man_paper_character))) "Hidden"))))

(fn `DamagCaculator`
  (bind _currenthealth (`self.CurrentHealth`))
  (if false
    (set `self.CurrentHealth` (- _currenthealth 1))
    (if (not (`self.Interrupted`))
      (set `self.Interrupted` true))
    (`KismetSystemLibrary.PrintString` (`KismetStringLibrary.Conv_IntToString` _currenthealth))))

(fn `GetGrabedNPC`
  (bind _aslizard_man_paper_character (cast `/Game/Blueprints/LizardMan_PaperCharacter` (`GameplayStatics.GetPlayerPawn` 0)))
  (if (`/Game/Blueprints/LizardMan_PaperCharacter.IsGrabing` _aslizard_man_paper_character)
    (`SceneComponent.K2_SetWorldLocation` (`self.Capsule`) (`SceneComponent.K2_GetComponentLocation` (`/Game/Blueprints/LizardMan_PaperCharacter.PunchBox` _aslizard_man_paper_character)) false false)))

(fn `GetLocationAtDistanceAlongSpline`
  (params (Target :type "SplineComponent Object Reference") (Distance :type "Float (double-precision)"))
  (returns (`Return Value` :type "Vector Structure"))
  (return (`SceneComponent.K2_GetComponentLocation` Target)))

(fn `Update Health`
  (params (Damage :type Integer))
  (bind _output_get (set `/Game/Blueprints/HPBar.HealthPercentage` (/ (`KismetMathLibrary.Conv_IntToDouble` (`self.CurrentHealth`)) (`KismetMathLibrary.Conv_IntToDouble` (`self.HP`))) (`self.HPBarWidget`)))
  (bind _ashpbar (cast `/Game/Blueprints/HPBar` (`WidgetComponent.GetUserWidgetObject` (`self.HPBar`))))
  (`ProgressBar.SetPercent` (`/Game/Blueprints/HPBar.ProgressBar_22` _ashpbar) _output_get))

(fn `UserConstructionScript`
  (`self.SetActorRotation` (struct :`Roll` -45.0))
  (bind _output_get (set `self.HP` (+ (* (`self.Level`) (`self.Willpower`)) (* (`self.Level`) (`self.Strength`)) (* (`self.Level`) (+ (`self.Strength`) (`self.Willpower`))) (* (`self.Level`) (+ (`self.Strength`) (`self.Willpower`) (`self.Stamina`))) (* (`self.Level`) (`self.Strength`)) (* (`self.Level`) (`self.Strength`)) (* (`self.Level`) (- (- (`self.Strength`) (`self.SelfControl`)) (`self.Money`))))))
  (set `self.CurrentHealth` _output_get))