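; SimpleSky is a day-night cycle actor that rotates the sun over a configurable day length.
; BeginPlay converts the day length in minutes into seconds per in-game hour.
; Each tick advances the hour, maps it to a sun pitch, sets the Sun actor's rotation and refreshes the SkyDome's sun direction, wrapping the hour to zero at 24.
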(event `self.ReceiveBeginPlay`
  (bind _output_get (set `self.OneDay` (* (`self.DayLenghtInMinutes`) 60.0)))
  (set `self.OneHour` (/ _output_get 24.0)))

(event `self.ReceiveTick`
  (params (DeltaSeconds :type "Float (single-precision)"))
  (bind _output_get (set `self.Hour` (+ (`self.Hour`) (/ DeltaSeconds (`self.OneHour`)))))
  (bind _output_get_2 (set `self.SunAngle` (+ (* (/ _output_get 6.0) 90.0) 90.0)))
  (`self.SetActorRotation` (`self.Sun`) (`KismetMathLibrary.MakeRotator` 0.0 _output_get_2))
  (`/Engine/EngineSky/BP_Sky_Sphere.UpdateSunDirection` (`self.SkyDome`))
  (if (>= (`self.Hour`) 24.0)
    (set `self.Hour` 0.0)))

(fn `UserConstructionScript`)