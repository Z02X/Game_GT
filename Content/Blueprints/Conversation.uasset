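; Conversation logic for dialogue between the lizard-man player and NPCs, displayed through the player's HPBarWidget.
; ConversationStart uses Enter to either call the widget's ProgressDialogue and HighlightChoice, or cast the player and NPC and blank the dialogue text fields.
; GetText holds hard-coded lines and four replies per stage for ConversationTestNPC.
; Its stage branches have constant false conditions and ignore DialogueNumber, so none of that text is currently returned.
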(fn ConversationStart
  (params (NPC :type Pawn%20Object%20Reference) (Enter :type Integer))
  (bind _slatecolor (Utilities|Struct|MakeSlateColor "(R=0.000000,G=0.000000,B=0.000000,A=1.000000)"))
  (if (== Enter 1)
    (Default|ProgressDialogue (Variables|/Game/Blueprints/LizardMan_PaperCharacter.LizardMan_PaperCharacter_C|GetHPBar%20Widget (stale _aslizard_man_paper_character)) (Variables|/Game/Blueprints/HPBar.HPBar_C|GetSelectedOption (Variables|/Game/Blueprints/LizardMan_PaperCharacter.LizardMan_PaperCharacter_C|GetHPBar%20Widget (stale _aslizard_man_paper_character))) (stale _asconversation_test_npc))
    (Default|HighlightChoice (Variables|/Game/Blueprints/LizardMan_PaperCharacter.LizardMan_PaperCharacter_C|GetHPBar%20Widget (stale _aslizard_man_paper_character)))
    (elif (== Enter 2)
      (Default|ProgressDialogue (Variables|/Game/Blueprints/LizardMan_PaperCharacter.LizardMan_PaperCharacter_C|GetHPBar%20Widget (stale _aslizard_man_paper_character)) 5 (stale _asconversation_test_npc))
      (Default|HighlightChoice (Variables|/Game/Blueprints/LizardMan_PaperCharacter.LizardMan_PaperCharacter_C|GetHPBar%20Widget (stale _aslizard_man_paper_character)))
      (elif (== Enter 3)
        (Default|ProgressDialogue (Variables|/Game/Blueprints/LizardMan_PaperCharacter.LizardMan_PaperCharacter_C|GetHPBar%20Widget (stale _aslizard_man_paper_character)) 6 (stale _asconversation_test_npc))
        (Default|HighlightChoice (Variables|/Game/Blueprints/LizardMan_PaperCharacter.LizardMan_PaperCharacter_C|GetHPBar%20Widget (stale _aslizard_man_paper_character)))
        (else
          (bind _aslizard_man_paper_character (Utilities|Casting|CastToLizardMan_PaperCharacter (Game|GetPlayerCharacter 0)))
          (Development|PrintString 0 (Utilities|String|ToString(Integer) 0))
          (bind _asconversation_test_npc (Utilities|Casting|CastToConversationTestNPC NPC))
          (Appearance|SetColorandOpacity (Variables|/Game/Blueprints/HPBar.HPBar_C|GetTxtNPC (Variables|/Game/Blueprints/LizardMan_PaperCharacter.LizardMan_PaperCharacter_C|GetHPBar%20Widget _aslizard_man_paper_character)) _slatecolor :!class /Script/UMG.TextBlock)
          (Rendering|Components|TextRender|SetText (Variables|/Game/Blueprints/HPBar.HPBar_C|GetTxtNPC (Variables|/Game/Blueprints/LizardMan_PaperCharacter.LizardMan_PaperCharacter_C|GetHPBar%20Widget _aslizard_man_paper_character)) "")
          (Appearance|SetColorandOpacity (Variables|/Game/Blueprints/HPBar.HPBar_C|GetTxtOpt1 (Variables|/Game/Blueprints/LizardMan_PaperCharacter.LizardMan_PaperCharacter_C|GetHPBar%20Widget _aslizard_man_paper_character)) _slatecolor :!class /Script/UMG.TextBlock)
          (Rendering|Components|TextRender|SetText (Variables|/Game/Blueprints/HPBar.HPBar_C|GetTxtOpt1 (Variables|/Game/Blueprints/LizardMan_PaperCharacter.LizardMan_PaperCharacter_C|GetHPBar%20Widget _aslizard_man_paper_character)) "")
          (Appearance|SetColorandOpacity (Variables|/Game/Blueprints/HPBar.HPBar_C|GetTxtOpt2 (Variables|/Game/Blueprints/LizardMan_PaperCharacter.LizardMan_PaperCharacter_C|GetHPBar%20Widget _aslizard_man_paper_character)) _slatecolor :!class /Script/UMG.TextBlock)
          (Rendering|Components|TextRender|SetText (Variables|/Game/Blueprints/HPBar.HPBar_C|GetTxtOpt2 (Variables|/Game/Blueprints/LizardMan_PaperCharacter.LizardMan_PaperCharacter_C|GetHPBar%20Widget _aslizard_man_paper_character)) "")
          (Appearance|SetColorandOpacity (Variables|/Game/Blueprints/HPBar.HPBar_C|GetTxtOpt3 (Variables|/Game/Blueprints/LizardMan_PaperCharacter.LizardMan_PaperCharacter_C|GetHPBar%20Widget _aslizard_man_paper_character)) _slatecolor :!class /Script/UMG.TextBlock)
          (Rendering|Components|TextRender|SetText (Variables|/Game/Blueprints/HPBar.HPBar_C|GetTxtOpt3 (Variables|/Game/Blueprints/LizardMan_PaperCharacter.LizardMan_PaperCharacter_C|GetHPBar%20Widget _aslizard_man_paper_character)) "")
          (Appearance|SetColorandOpacity (Variables|/Game/Blueprints/HPBar.HPBar_C|GetTxtOpt4 (Variables|/Game/Blueprints/LizardMan_PaperCharacter.LizardMan_PaperCharacter_C|GetHPBar%20Widget _aslizard_man_paper_character)) _slatecolor :!class /Script/UMG.TextBlock)
          (Rendering|Components|TextRender|SetText (Variables|/Game/Blueprints/HPBar.HPBar_C|GetTxtOpt4 (Variables|/Game/Blueprints/LizardMan_PaperCharacter.LizardMan_PaperCharacter_C|GetHPBar%20Widget _aslizard_man_paper_character)) ""))))))

(fn GetText
  (params (NPC :type Pawn%20Object%20Reference) (DialogueNumber :type String))
  ;[1 1 1] Npc Type Branches
  (if (== NPC "/Game/Blueprints/ConversationTestNPC.ConversationTestNPC")
    ;[1 1 1] ConversationTestNPC Text
    (if false
      (LocalVariables|SetReturn0 "Hi, I'm an NPC!")
      (LocalVariables|SetReturn1 "Hi, I'm the player!")
      (LocalVariables|SetReturn2 "Where are we?")
      (LocalVariables|SetReturn3 "Go away!")
      (LocalVariables|SetReturn4 "Can you give me some directions?")
      (return (LocalVariables|GetReturn0) (LocalVariables|GetReturn1) (LocalVariables|GetReturn2) (LocalVariables|GetReturn3) (LocalVariables|GetReturn4))
      (elif false
        (LocalVariables|SetReturn0 "It's nice to meet you, Player.")
        (LocalVariables|SetReturn1 "It's nice to meet you, too.")
        (LocalVariables|SetReturn2 "It's horrible to meet you.")
        (LocalVariables|SetReturn3 "Where are we?")
        (LocalVariables|SetReturn4 "What's your name?")
        (return (LocalVariables|GetReturn0) (LocalVariables|GetReturn1) (LocalVariables|GetReturn2) (LocalVariables|GetReturn3) (LocalVariables|GetReturn4))
        (elif false
          (LocalVariables|SetReturn0 "Now, what can I do for you?")
          (LocalVariables|SetReturn1 "Nothing right now, thanks.")
          (LocalVariables|SetReturn2 "Have you heard of the Super Secret Base?")
          (LocalVariables|SetReturn3 "Your face, bub.")
          (LocalVariables|SetReturn4 "Can you give me directions to the bus station?")
          (return (LocalVariables|GetReturn0) (LocalVariables|GetReturn1) (LocalVariables|GetReturn2) (LocalVariables|GetReturn3) (LocalVariables|GetReturn4))
          (elif (== 0 100)
            (LocalVariables|SetReturn0 "Why, this is Asteroid City 2234E!")
            (LocalVariables|SetReturn1 "Is this an important city?")
            (LocalVariables|SetReturn2 "Well, it sucks.")
            (LocalVariables|SetReturn3 "Do you live here?")
            (LocalVariables|SetReturn4 "It looks cool.")
            (return (LocalVariables|GetReturn0) (LocalVariables|GetReturn1) (LocalVariables|GetReturn2) (LocalVariables|GetReturn3) (LocalVariables|GetReturn4))))))))