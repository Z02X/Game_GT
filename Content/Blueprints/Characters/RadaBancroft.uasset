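; Rada Bancroft is an NPC that walks a spline on a daily routine driven by the SimpleSky hour and can be hurt or carried by the player.
; Each tick, hour and distance gates advance it along the spline, with a line trace setting its height.
; Player overlap drains health, or snaps the capsule to the player's PunchBox while grabbing.
; Construction derives HP from level and stats, and UpdateHealth feeds the health bar widget.
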(event `self.ReceiveBeginPlay`
  ;[1 1 1] Branches
  (bind _returnvalue (`|CreateWidget` "/Game/Blueprints/HPBar.HPBar_C"))
  (set `self.HPBarWidget` _returnvalue)
  (bind _output_get (set `self.StartingLocation` (`self.K2_GetActorLocation`))))

(event `self.ReceiveTick`
  (params (DeltaSeconds :type "Float (single-precision)"))
  (bind _current_location (`self.Current Location`))
  ;[1 1 1] Update Health
  (`self.Update Health` 0)
  (bind _assimple_sky (cast `/Game/Blueprints/SimpleSky` (`self.SkyControlerRef`)))
  (bind _output_get (set `self.LocalHour` (`/Game/Blueprints/SimpleSky.Hour` _assimple_sky)))
  (if (`self.IsOverlappingActor` (`GameplayStatics.GetPlayerPawn` 0))
    (`self.DamagCaculator`)
    (`self.GetGrabedNPC`)
    (if (not (`self.Interrupted`))
      (set `self.Interrupted` true)
      ;[1 1 1] Branches
      (if (>= (`self.DistanceAlongSpline`) 100000.0) :!label _label
        (if (not (>= (`self.LocalHour`) 4.749))
          (set `self.DistanceAlongSpline` 0.0)
          (`self.K2_SetActorLocation` (stale `self.ReceiveBeginPlay` _output_get))
          (if (>= _output_get 4.75) :!label _label_2
            (if (>= (`self.DistanceAlongSpline`) 600.0)
              (if (>= (`self.LocalHour`) 18.0)
                (if (>= (`self.DistanceAlongSpline`) 1200.0)
                  (if (>= (`self.LocalHour`) 19.0)
                    ;[1 1 1] Normal Routines everything else leads to
                    (set `self.DistanceAlongSpline` (+ (`self.Speed`) (`self.DistanceAlongSpline`)) :!label _label_3)
                    (set `self.Current Location` (`SplineComponent.GetLocationAtDistanceAlongSpline` (`/Game/Blueprints/SplineComponet.Spline` (`self.Spline_Blueprint`)) (`self.DistanceAlongSpline`) "World"))
                    (bind _outhit (`KismetSystemLibrary.LineTraceSingleForObjects` _current_location (`KismetMathLibrary.MakeVector` (.x _current_location) (.y _current_location) 20.0) (`|MakeArray` "ObjectTypeQuery4" :!type "EObjectTypeQuery Enum")))
                    (set `self.Trace Hit Location` (`.ImpactPoint` (`GameplayStatics.BreakHitResult` _outhit)))
                    (`self.K2_SetActorLocation` (`KismetMathLibrary.MakeVector` (.x (`self.Current Location`)) (.y (`self.Current Location`)) (+ (.z (`self.Trace Hit Location`)) 20.0))))
                  (else
                    (goto _label_3))))
              (else
                (goto _label_3)))))
        (elif (not (`self.Interrupted`))
          (goto _label_2))))
    (else
      (goto _label))))

(fn `DamagCaculator`
  (bind _returnvalue (`GameplayStatics.GetPlayerPawn` 0))
  (bind _currenthealth (`self.CurrentHealth`))
  (if (`self.IsOverlappingActor` _returnvalue)
    (bind _aslizard_man_paper_character (cast `/Game/Blueprints/LizardMan_PaperCharacter` _returnvalue))
    (if (not (`/Game/Blueprints/LizardMan_PaperCharacter.IsGrabing` _aslizard_man_paper_character))
      (set `self.CurrentHealth` (- _currenthealth 1))
      (if (not (`self.Interrupted`))
        (set `self.Interrupted` true))
      (`KismetSystemLibrary.PrintString` (`KismetStringLibrary.Conv_IntToString` _currenthealth)))))

(fn `GetGrabedNPC`
  (bind _aslizard_man_paper_character (cast `/Game/Blueprints/LizardMan_PaperCharacter` (`GameplayStatics.GetPlayerPawn` 0)))
  (if (`/Game/Blueprints/LizardMan_PaperCharacter.IsGrabing` _aslizard_man_paper_character)
    (`SceneComponent.K2_SetWorldLocation` (`self.Capsule`) (`SceneComponent.K2_GetComponentLocation` (`/Game/Blueprints/LizardMan_PaperCharacter.PunchBox` _aslizard_man_paper_character)) false false)))

(fn `GetLocationAtDistanceAlongSpline`
  (params (Target :type "SplineComponent Object Reference") (Distance :type "Float (double-precision)"))
  (returns (`Return Value` :type "Vector Structure"))
  (return (`SceneComponent.K2_GetComponentLocation` Target)))

(fn `Update Health`
  (params (Damage :type Integer))
  (bind _output_get (set `/Game/Blueprints/HPBar.HealthPercentage` (/ (`KismetMathLibrary.Conv_IntToDouble` (`self.CurrentHealth`)) (`KismetMathLibrary.Conv_IntToDouble` (`self.HP`))) (`self.HPBarWidget`)))
  (bind _ashpbar (cast `/Game/Blueprints/HPBar` (`WidgetComponent.GetUserWidgetObject` (`self.HPBar`))))
  (`ProgressBar.SetPercent` (`/Game/Blueprints/HPBar.ProgressBar_22` _ashpbar) _output_get))

(fn `UserConstructionScript`
  (`self.SetActorRotation` (struct :`Roll` -45.0))
  (bind _output_get (set `self.HP` (+ (* (`self.Level`) (`self.Willpower`)) (* (`self.Level`) (`self.Strength`)) (* (`self.Level`) (+ (`self.Strength`) (`self.Willpower`))) (* (`self.Level`) (+ (`self.Strength`) (`self.Willpower`) (`self.Stamina`))) (* (`self.Level`) (`self.Strength`)) (* (`self.Level`) (`self.Strength`)) (* (`self.Level`) (- (- (`self.Strength`) (`self.SelfControl`)) (`self.Money`))))))
  (set `self.CurrentHealth` _output_get))