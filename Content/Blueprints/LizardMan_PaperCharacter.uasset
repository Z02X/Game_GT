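; LizardMan is a Paper2D player character with planar movement, a timed punch and a hold-to-grab action, its actor tilted 45 degrees at construction.
; Primary briefly enables the PunchBox collision, while Secondary keeps it enabled until release.
; Horizontal input flips the sprite and Arrow1 to face travel, except while grabbing.
; Weapon ID switches have no branches wired, and the Arrow1 bullet spawn is disconnected.
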(event `InputAction|Secondary`
  (params (Key :type "Key Structure" :default "AnyKey"))
  (bind _punchbox (`self.PunchBox`))
  (:`Pressed`
    (switch `int` (`self.Wepon_ID`)
      (:`0`
        (set `self.IsGrabing` true)
        (`SceneComponent.SetHiddenInGame` _punchbox false false)
        (`PrimitiveComponent.SetCollisionEnabled` _punchbox "QueryOnly"))))
  (:`Released`
    (switch `int` 0
      (:`0`
        (set `self.IsGrabing` false)
        (`SceneComponent.SetHiddenInGame` _punchbox true false)
        (`PrimitiveComponent.SetCollisionEnabled` _punchbox "NoCollision")))))

(event `InputAxis|MoveHorizontally`
  (params (AxisValue :type "Float (single-precision)"))
  (bind _arrow1 (`self.Arrow1`))
  (bind _sprite (`self.Sprite`))
  (`self.AddMovementInput` (0.2 0.0 0.0) AxisValue)
  (if (< AxisValue 0.0)
    (if (not (`self.IsGrabing`))
      (`SceneComponent.K2_SetRelativeRotation` _sprite (struct :`Yaw` 180.0) false false)
      (`SceneComponent.K2_SetRelativeTransform` _arrow1 (`KismetMathLibrary.Conv_VectorToTransform` (-10.0 3.0 -1.5)) false false)
      (`SceneComponent.K2_SetRelativeRotation` _arrow1 (struct :`Yaw` -180.0) false false))
    (elif (> AxisValue 0.0)
      (if (not (`self.IsGrabing`))
        (`SceneComponent.K2_SetRelativeRotation` _sprite (struct) false false)
        (`SceneComponent.K2_SetRelativeTransform` _arrow1 (`KismetMathLibrary.Conv_VectorToTransform` (10.0 3.0 -1.5)) false false)
        (`SceneComponent.K2_SetRelativeRotation` _arrow1 (struct) false false)))))

(event `InputAction|Primary`
  (params (Key :type "Key Structure" :default "AnyKey"))
  (bind _punchbox (`self.PunchBox`))
  (:`Pressed`
    (switch `int` (`self.Wepon_ID`)
      (:`0`
        (`SceneComponent.SetHiddenInGame` _punchbox false false)
        (`PrimitiveComponent.SetCollisionEnabled` _punchbox "QueryOnly")
        (`KismetSystemLibrary.Delay` 0.4)
        (`SceneComponent.SetHiddenInGame` _punchbox true false)
        (`PrimitiveComponent.SetCollisionEnabled` _punchbox "NoCollision")))))

(event `InputAxis|MoveVertically`
  (params (AxisValue :type "Float (single-precision)"))
  (`self.AddMovementInput` (0.0 0.2 0.0) AxisValue))

(fn `UserConstructionScript`
  (`self.SetActorRotation` (struct :`Roll` -45.0))
  (`PrimitiveComponent.SetCollisionEnabled` (`self.PunchBox`) "NoCollision"))