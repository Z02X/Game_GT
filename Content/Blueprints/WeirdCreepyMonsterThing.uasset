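; Creature actor that moves along the spline of a referenced SplineBlueprint while snapping to static world geometry beneath it.
; Each Tick advances the spline distance by Speed, without delta-time scaling, and samples that world location.
; A persistently drawn object trace runs from there to world Z zero, and the actor moves to its impact point without checking for a hit.
; A local GetLocationAtDistanceAlongSpline function ignores Distance.
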(event `self.ReceiveTick`
  (params (DeltaSeconds :type "Float (single-precision)"))
  (bind _current_location (`self.Current Location`))
  (set `self.DistanceAlongSpline` (+ (`self.Speed`) (`self.DistanceAlongSpline`)))
  (set `self.Current Location` (`SplineComponent.GetLocationAtDistanceAlongSpline` (`/Game/Blueprints/SplineComponet.Spline` (`self.Spline_Blueprint`)) (`self.DistanceAlongSpline`) "World"))
  (bind _outhit (`KismetSystemLibrary.LineTraceSingleForObjects` :`Start` _current_location :`End` (`KismetMathLibrary.MakeVector` (.x _current_location) (.y _current_location) 0.0) :`ObjectTypes` (`|MakeArray` "ObjectTypeQuery1" :!type "EObjectTypeQuery Enum") :`DrawDebugType` "Persistent"))
  (bind _output_get (set `self.Trace Hit Location` (`.ImpactPoint` (`GameplayStatics.BreakHitResult` _outhit))))
  (`self.K2_SetActorLocation` _output_get))

(fn `GetLocationAtDistanceAlongSpline`
  (params (Target :type "SplineComponent Object Reference") (Distance :type "Float (double-precision)"))
  (returns (`Return Value` :type "Vector Structure"))
  (return (`SceneComponent.K2_GetComponentLocation` Target)))

(fn `UserConstructionScript`)