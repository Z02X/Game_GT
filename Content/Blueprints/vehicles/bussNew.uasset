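; Bus vehicle that drives along numbered waypoints and also carries NPC-style dialogue logic.
; In movement mode 0, Tick runs Comute, which steers toward the VehicleTargetPoint matching the current ID and increments it on capsule overlap, without wrapping.
; Sphere overlap with a DialogueBox starts a test conversation and shows the player's HUD dialogue options; the player leaving hides them.
; Steering divides the XY offset by squared distance rather than normalizing it.
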(event `/Game/TestContent/CharacterTest1.ReceiveBeginPlay`)

(event `self.ReceiveActorBeginOverlap`
  (params (OtherActor :type "Actor Object Reference")))

(event `self.Sphere.OnComponentEndOverlap`
  (params (OtherActor :type "Actor Object Reference") (OtherComp :type "PrimitiveComponent Object Reference") (OtherBodyIndex :type Integer))
  (`self.Overlap` false OtherActor))

(event `self.Sphere.OnComponentBeginOverlap`
  (params (OtherActor :type "Actor Object Reference") (OtherComp :type "PrimitiveComponent Object Reference") (OtherBodyIndex :type Integer) (bFromSweep :type Boolean) (SweepResult :type "HitResult Structure (by ref)"))
  (`self.Overlap` true OtherActor))

(event `/Game/TestContent/CharacterTest1.ReceiveTick`
  (params (DeltaSeconds :type "Float (single-precision)"))
  (switch `int` (`self.MovementMode`)
    (:`0`
      (`self.Comute`)
      (if (== (`GameplayStatics.GetObjectClass` (stale `self.Sphere.OnComponentBeginOverlap` OtherActor)) "/Game/Blueprints/DialogueBox.DialogueBox_C")
        (bind _aslizard_man_paper_character (cast `/Game/Blueprints/LizardMan_PaperCharacter` (`GameplayStatics.GetPlayerCharacter` 0)))
        (`Widget.SetKeyboardFocus` (`/Game/Blueprints/LizardMan_PaperCharacter.HPBar Widget` _aslizard_man_paper_character))))))

(event `Key|Enter`
  (params (Key :type "Key Structure" :default "AnyKey"))
  (:`Pressed`
    (`KismetSystemLibrary.PrintText` "Hello")))

(fn `Comute`
  (bind _outactors (`GameplayStatics.GetAllActorsOfClass` "/Game/TestContent/VehicleTargetPoint.VehicleTargetPoint_C"))
  (for _array_element _outactors
    (if (== (`self.CurentTargetWaypoint`) (`/Game/TestContent/VehicleTargetPoint.ID` _array_element))
      (if (`PrimitiveComponent.IsOverlappingComponent` (`self.CapsuleComponent`) (`/Game/TestContent/VehicleTargetPoint.Capsule` _array_element))
        (bind _idout (`self.WaypointOrder_Controller` (`self.CurentTargetWaypoint`)))
        (set `self.CurentTargetWaypoint` _idout)
        (else
          (bind _returnvalue (- (.x (`self.K2_GetActorLocation` _array_element)) (.x (`SceneComponent.K2_GetComponentLocation` (`self.CapsuleComponent`)))))
          (bind _returnvalue_2 (- (.y (`self.K2_GetActorLocation` _array_element)) (.y (`SceneComponent.K2_GetComponentLocation` (`self.CapsuleComponent`)))))
          (bind _returnvalue_3 (+ (`KismetMathLibrary.Square` _returnvalue) (`KismetMathLibrary.Square` _returnvalue_2)))
          (`self.AddMovementInput` (`KismetMathLibrary.MakeVector` (/ _returnvalue _returnvalue_3) (/ _returnvalue_2 _returnvalue_3)) 10.0))))))

(fn `Overlap`
  (params (OverlapBegin :type Boolean) (OtherActor :type "Actor Object Reference"))
  (bind _returnvalue (`GameplayStatics.GetPlayerCharacter` 0))
  (bind _emptytext (`self.EmptyText`))
  (if OverlapBegin
    (if (== (`GameplayStatics.GetObjectClass` OtherActor) "/Game/Blueprints/DialogueBox.DialogueBox_C")
      (bind _aslizard_man_paper_character (cast `/Game/Blueprints/LizardMan_PaperCharacter` _returnvalue))
      (bind _hpbar_widget (`/Game/Blueprints/LizardMan_PaperCharacter.HPBar Widget` _aslizard_man_paper_character))
      (bind _image_36 (`/Game/Blueprints/HPBar.Image_36` _hpbar_widget))
      (`Widget.SetVisibility` _image_36 "Visible")
      (`/Game/Blueprints/Conversation.ConversationStart` self 0 "CharacterTest1")
      (bind _txtnpc (`/Game/Blueprints/HPBar.TxtNPC` _hpbar_widget))
      (`Widget.SetVisibility` _txtnpc "Visible")
      (bind _txtopt1 (`/Game/Blueprints/HPBar.TxtOpt1` _hpbar_widget))
      (`Widget.SetVisibility` _txtopt1 "Visible")
      (bind _btnopt1 (`/Game/Blueprints/HPBar.BtnOpt1` _hpbar_widget))
      (`Widget.SetVisibility` _btnopt1 "Visible")
      (bind _txtopt2 (`/Game/Blueprints/HPBar.TxtOpt2` _hpbar_widget))
      (if (`KismetTextLibrary.NotEqual_TextText` (`TextBlock.GetText` _txtopt2) _emptytext)
        (`Widget.SetVisibility` _txtopt2 "Visible")
        (bind _btnopt2 (`/Game/Blueprints/HPBar.BtnOpt2` _hpbar_widget))
        (`Widget.SetVisibility` _btnopt2 "Visible")
        (bind _txtopt3 (`/Game/Blueprints/HPBar.TxtOpt3` _hpbar_widget))
        (if (`KismetTextLibrary.NotEqual_TextText` (`TextBlock.GetText` _txtopt3) _emptytext)
          (`Widget.SetVisibility` _txtopt3 "Visible")
          (bind _btnopt3 (`/Game/Blueprints/HPBar.BtnOpt3` _hpbar_widget))
          (`Widget.SetVisibility` _btnopt3 "Visible")
          (bind _txtopt4 (`/Game/Blueprints/HPBar.TxtOpt4` _hpbar_widget))
          (if (`KismetTextLibrary.NotEqual_TextText` (`TextBlock.GetText` _txtopt4) _emptytext)
            (`Widget.SetVisibility` _txtopt4 "Visible")
            (bind _btnopt4 (`/Game/Blueprints/HPBar.BtnOpt4` _hpbar_widget))
            (`Widget.SetVisibility` _btnopt4 "Visible")))))
    (elif (== OtherActor _returnvalue)
      (set `/Game/Blueprints/HPBar.DialogueNumber` "" _hpbar_widget)
      (`Widget.SetVisibility` _image_36 "Hidden")
      (`Widget.SetVisibility` _txtnpc "Hidden")
      (`Widget.SetVisibility` _txtopt1 "Hidden")
      (`Widget.SetVisibility` _btnopt1 "Hidden")
      (`Widget.SetVisibility` _txtopt2 "Hidden")
      (`Widget.SetVisibility` _btnopt2 "Hidden")
      (`Widget.SetVisibility` _txtopt3 "Hidden")
      (`Widget.SetVisibility` _btnopt3 "Hidden")
      (`Widget.SetVisibility` _txtopt4 "Hidden")
      (`Widget.SetVisibility` _btnopt4 "Hidden")
      (`KismetSystemLibrary.PrintString` "Hello"))))

(fn `UserConstructionScript`)

(fn `WaypointOrder_Controller`
  (params (IdIn :type Integer))
  (returns (IdOut :type Integer))
  (return (+ IdIn 1)))